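; Shielded_Enemy is an enemy actor whose Cylinder component, apparently its shield, blocks or opens based on player proximity.
; When PlayerCharacter_BP begins overlapping OuterCollision, the Cylinder's collision is disabled.
; When the player leaves, a short delay runs before the Cylinder's query and physics collision is restored.
; Tick, BeginPlay and the construction script add no logic of their own.
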(event `self.OuterCollision.OnComponentBeginOverlap`
  (params (OverlappedComponent :type "PrimitiveComponent Object Reference") (OtherActor :type "Actor Object Reference") (OtherComp :type "PrimitiveComponent Object Reference") (OtherBodyIndex :type Integer) (bFromSweep :type Boolean) (SweepResult :type "HitResult Structure (by ref)"))
  (cast `/Game/Blueprints/Character/PlayerCharacter_BP` OtherActor)
  (`PrimitiveComponent.SetCollisionEnabled` (`self.Cylinder`) "NoCollision"))

(event `self.OuterCollision.OnComponentEndOverlap`
  (params (OverlappedComponent :type "PrimitiveComponent Object Reference") (OtherActor :type "Actor Object Reference") (OtherComp :type "PrimitiveComponent Object Reference") (OtherBodyIndex :type Integer))
  (cast `/Game/Blueprints/Character/PlayerCharacter_BP` OtherActor)
  (`KismetSystemLibrary.Delay` 0.2)
  (`PrimitiveComponent.SetCollisionEnabled` (`self.Cylinder`) "QueryAndPhysics"))

(fn `UserConstructionScript`
  (`parent.UserConstructionScript`))