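; Player character Blueprint that dashes along its Cube's forward vector and ricochets off BounceWall actors.
; Fast enough wall hits mirror the stored dash vector by the hit normal and relaunch, with strength derived from DashSpeed, a growing bounce count and current speed.
; A DoOnce reset after a short delay debounces hits.
; The Break input plays a timeline that yaws the Cube, then resets its rotation after a delay.
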(event `InputAction|Break`
  (params (Key :type "Key Structure" :default "AnyKey"))
  (bind _cube (`self.Cube`))
  (:`Pressed`
    (bind (_direction _newtrack_0) (`Timeline|Timeline_0` :!via `PlayFromStart`)
      (:`Update`
        (`SceneComponent.K2_AddLocalRotation` _cube (`KismetMathLibrary.MakeRotator` 0.0 0.0 _newtrack_0) false false)
        (`KismetSystemLibrary.Delay` 0.3)
        (`SceneComponent.K2_SetRelativeRotation` :`self` _cube)))))

(event `InputAction|Dash`
  (params (Key :type "Key Structure" :default "AnyKey"))
  (bind _returnvalue (`SceneComponent.GetForwardVector` (`self.Cube`)))
  (:`Pressed`
    (set `self.BounceCount` 1.0)
    (set `self.Current Vector` _returnvalue)
    (`self.LaunchCharacter` (* _returnvalue (`self.DashSpeed`)) true true)))

(event `self.ReceiveHit`
  (params (MyComp :type "PrimitiveComponent Object Reference") (Other :type "Actor Object Reference") (OtherComp :type "PrimitiveComponent Object Reference") (bSelfMoved :type Boolean) (HitLocation :type "Vector Structure") (HitNormal :type "Vector Structure") (NormalImpulse :type "Vector Structure") (Hit :type "HitResult Structure (by ref)"))
  (bind _returnvalue (`KismetMathLibrary.MirrorVectorByNormal` (`self.Current Vector`) HitNormal))
  (cast `/Game/Blueprints/BounceWall` Other)
  (if (>= (`KismetMathLibrary.Abs` (`KismetMathLibrary.VSize` (`self.GetVelocity`))) 300.0)
    (set `self.BounceCount` (+ (`self.BounceCount`) 0.5))
    (`/Engine/EditorBlueprintResources/StandardMacros.DoOnce` false :!label _label
      (:`Completed`
        (`self.LaunchCharacter` (* _returnvalue (`KismetMathLibrary.Abs` (- (/ (`self.DashSpeed`) (`self.BounceCount`)) (`KismetMathLibrary.Abs` (`KismetMathLibrary.VSize` (`self.GetVelocity`)))))) true true)
        (`KismetSystemLibrary.Delay` 0.1)
        (`self.ResetBounce`)
        (set `self.Current Vector` _returnvalue)
        (`KismetSystemLibrary.PrintString` (`KismetStringLibrary.Conv_DoubleToString` (`self.BounceCount`)))))))

(event `ResetBounce`
  (goto _label :!via `Reset`))

(fn `UserConstructionScript`)