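; Physics-driven character Blueprint that dashes along its Cube's forward vector and ricochets off BounceWall actors.
; Dash applies a capsule impulse and stores the direction, while Break plays a timeline that yaws the Cube, with delayed resets to zero rotation.
; Wall hits launch the character along the mirrored direction at current speed, debounced by a DoOnce that resets after a short delay.
; ForceDash offers a continuous-force alternative, uncalled here.
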(event `InputAction|Dash`
  (params (Key :type "Key Structure" :default "AnyKey"))
  (bind _returnvalue (`SceneComponent.GetForwardVector` (`self.Cube`)))
  (:`Pressed`
    (set `self.Current Vector` _returnvalue)
    (`PrimitiveComponent.AddImpulse` (`self.CapsuleComponent`) (* _returnvalue (`self.DashSpeed`)) "None" false)))

(event `InputAction|Break`
  (params (Key :type "Key Structure" :default "AnyKey"))
  (bind _cube (`self.Cube`))
  (:`Pressed`
    (bind (_direction _newtrack_0) (`Timeline|Timeline_0` :!via `PlayFromStart`)
      (:`Update`
        (`SceneComponent.K2_AddLocalRotation` _cube (`KismetMathLibrary.MakeRotator` 0.0 0.0 _newtrack_0) false false)
        (`KismetSystemLibrary.Delay` 0.3)
        (`SceneComponent.K2_SetRelativeRotation` :`self` _cube)))))

(event `InputAction|Dash`
  (params (Key :type "Key Structure" :default "AnyKey")))

(event `self.ReceiveHit`
  (params (MyComp :type "PrimitiveComponent Object Reference") (Other :type "Actor Object Reference") (OtherComp :type "PrimitiveComponent Object Reference") (bSelfMoved :type Boolean) (HitLocation :type "Vector Structure") (HitNormal :type "Vector Structure") (NormalImpulse :type "Vector Structure") (Hit :type "HitResult Structure (by ref)"))
  (bind _returnvalue (`KismetMathLibrary.MirrorVectorByNormal` (`self.Current Vector`) HitNormal))
  (bind _asbounce_wall (cast `/Game/Blueprints/BounceWall` Other))
  (`/Engine/EditorBlueprintResources/StandardMacros.DoOnce` false :!label _label
    (:`Completed`
      (`KismetSystemLibrary.PrintString` (`KismetSystemLibrary.GetDisplayName` _asbounce_wall))
      (`self.LaunchCharacter` (* _returnvalue (`KismetMathLibrary.VSize` (`self.GetVelocity`))) true true)
      (`KismetSystemLibrary.Delay` 0.2)
      (`self.ResetBounce`)
      (set `self.Current Vector` _returnvalue))))

(event `ResetBounce`
  (goto _label :!via `Reset`))

(fn `ForceDash`
  (`PrimitiveComponent.AddForce` (`self.CapsuleComponent`) (* (`self.Current Vector`) (`self.DashSpeed`)) "None" true))

(fn `UserConstructionScript`)